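; Unfinished game mode for a carpentry game, meant to generate customer orders periodically.
; BeginPlay starts a looping timer calling GenerateNewOrder, with an interval randomized once between min and max settings.
; GenerateNewOrder and AddOrder are empty, with disconnected nodes for picking a random AvailableOrders data table row and appending to CurrentOrders.
; An unwired cast also expects this game mode class from GetGameState.
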(event Custom|GenerateNewOrder)

(event EventBeginPlay
  (Utilities|Time|SetTimerbyFunctionName 0 "GenerateNewOrder" (Math|Random|RandomFloatinRange (Variables|Default|GetOrderGenerationTimeMin) (Variables|Default|GetOrderGenerationTimeMax)) true))

(event EventTick
  (params (DeltaSeconds :type Float%20%28single-precision%29)))

(fn ConstructionScript)

(fn GenerateNewOrder)

(fn AddOrder
  (params (NewOrder :type Struct%20Order%20Structure)))